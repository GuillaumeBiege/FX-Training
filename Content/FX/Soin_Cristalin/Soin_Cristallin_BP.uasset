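; Timeline-style effect actor for a crystal healing visual (Soin Cristallin), combining a ground decal, six flying crystals and ground crystals.
; BeginPlay creates a dynamic material for the decal, and Tick accumulates Time and feeds it to that material's Time parameter.
; The same clock activates each flying crystal at its own time from an array, and the ground crystals at theirs, with flags making each activation one-shot.
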(event EventBeginPlay
  (CallFunction|SetDynamicMat))

(event Collision|EventActorBeginOverlap
  (params (OtherActor :type Actor%20Object%20Reference)))

(event EventTick
  (params (DeltaSeconds :type Float%20%28single-precision%29))
  (Variables|Default|SetTime (+ DeltaSeconds (Variables|Default|GetTime)))
  (CallFunction|GroundEffectUpdate)
  (FlyingCristals|FlyingCristalsUpdate)
  (Groundcristal|GroundCrystalUpdate))

(fn ConstructionScript)

(fn GroundEffectUpdate
  (Rendering|Material|SetScalarParameterValue (Variables|Material|GetGroundEffectDynamicMat) "Time" (Variables|Default|GetTime) :!class /Script/Engine.MaterialInstanceDynamic))

(fn SetDynamicMat
  (bind _returnvalue (Rendering|Material|CreateDynamicMaterialInstance (Variables|Default|GetDecal) :!class /Script/Engine.DecalComponent))
  (Variables|Material|SetGroundEffectDynamicMat _returnvalue))

(fn FlyingCristalsUpdate
  (bind _index (Utilities|FlowControl|ForLoopwithBreak 0 5)
    (:LoopBody
      (switch int _index
        (:0
          (bind _isittime (FlyingCristals|CheckTimeFlyingCristalActivation (Variables|Default|GetTime) _index))
          (if _isittime
            (Components|Activation|Activate (Variables|Default|GetFlyingCrystal_1) false)))
        (:1
          (bind _isittime_2 (FlyingCristals|CheckTimeFlyingCristalActivation (Variables|Default|GetTime) _index))
          (if _isittime_2
            (Components|Activation|Activate (Variables|Default|GetFlyingCrystal_2) false)))
        (:2
          (bind _isittime_3 (FlyingCristals|CheckTimeFlyingCristalActivation (Variables|Default|GetTime) _index))
          (if _isittime_3
            (Components|Activation|Activate (Variables|Default|GetFlyingCrystal_3) false)))
        (:3
          (bind _isittime_4 (FlyingCristals|CheckTimeFlyingCristalActivation (Variables|Default|GetTime) _index))
          (if _isittime_4
            (Components|Activation|Activate (Variables|Default|GetFlyingCrystal_4) false)))
        (:4
          (bind _isittime_5 (FlyingCristals|CheckTimeFlyingCristalActivation (Variables|Default|GetTime) _index))
          (if _isittime_5
            (Components|Activation|Activate (Variables|Default|GetFlyingCrystal_5) false)))
        (:5
          (bind _isittime_6 (FlyingCristals|CheckTimeFlyingCristalActivation (Variables|Default|GetTime) _index))
          (if _isittime_6
            (Components|Activation|Activate (Variables|Default|GetFlyingCrystal_6) false)))))))

(fn CheckTimeFlyingCristalActivation
  (params (Time :type Float%20%28double-precision%29) (Index :type Integer))
  (if (not (Utilities|Array|Get(acopy) (Variables|FlyingCristals|GetIsActivated) Index))
    (if (>= Time (Utilities|Array|Get(acopy) (Variables|FlyingCristals|GetActivationTime) Index))
      (Utilities|Array|SetArrayElem (Variables|FlyingCristals|GetIsActivated) Index true)
      (return true)
      (else
        (return false)))))

(fn GroundCrystalUpdate
  (if (not (Variables|Groundcristal|GetGroundCristalIsActivated))
    (if (>= (Variables|Default|GetTime) (Variables|Groundcristal|GetGroundCristalActivationTime))
      (Variables|Groundcristal|SetGroundCristalIsActivated true)
      (Components|Activation|Activate (Variables|Default|GetGround_Crystals) false))))