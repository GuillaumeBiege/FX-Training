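; Summoning circle VFX actor for a Hand of Gul'dan effect: runic circles, a portal, a fel beam and a falling demonic meteor.
; Tick accumulates Time, which gates each stage and samples curves driving dynamic material parameters and portal scale.
; The beam and meteor run normalized timers through curves to lerp toward their end points.
; On arrival the meteor triggers an explosion and delayed destruction; the actor destroys itself after a set lifetime.
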(event Custom|SpawnExplosion
  (params (Position :type Vector))
  (Components|Activation|Activate (Variables|Default|GetExplosion) false))

(event EventBeginPlay
  (Material|SetDynamicMat))

(event Collision|EventActorBeginOverlap
  (params (OtherActor :type Actor%20Object%20Reference)))

(event EventTick
  (params (DeltaSeconds :type Float%20%28single-precision%29))
  (Variables|Default|SetTime (+ DeltaSeconds (Variables|Default|GetTime)))
  (CallFunction|CheckAutoDestroy)
  (Beam|SpawnBeam DeltaSeconds)
  (Material|UpdateDynamicMat)
  (if (Variables|Portal|GetIsVisible)
    (Transformation|SetRelativeScale3D (Variables|Default|GetPortal) (* "10.000000,10.000000,10.000000" (Math|Curves|GetFloatValue (Variables|Portal|GetCurvePortalSize) (Variables|Default|GetTime)))))
  (CallFunction|PortalVisibility)
  (if (< (Variables|Meteor|GetTimerMeteorTravel) 1.0)
    (bind _bool (Meteor|SpawnMeteor))
    (if _bool
      (if (Variables|Meteor|GetIsMeteorSpawned)
        (Meteor|MoveMeteor DeltaSeconds)
        (Meteor|DestroyMeteor)))))

(fn ConstructionScript)

(fn PortalVisibility
  (if (Variables|Portal|GetIsPortalSpawed)
    (if (Variables|Portal|GetIsVisible)
      (if (> (Variables|Default|GetTime) (Variables|Portal|GetTimePortalDispawn))
        (Rendering|SetVisibility (Variables|Default|GetPortal) false false)
        (Variables|Portal|SetIsVisible false)))
    (elif (not (Variables|Portal|GetIsVisible))
      (if (> (Variables|Default|GetTime) (Variables|Portal|GetTimePortalSpawn))
        (Variables|Portal|SetIsPortalSpawed true)
        (Rendering|SetVisibility (Variables|Default|GetPortal) true false)
        (Variables|Portal|SetIsVisible true)))))

(fn SetDynamicMat
  (bind _returnvalue (Rendering|Material|CreateDynamicMaterialInstance (Variables|Default|GetCercleExterieur) :!class /Script/Engine.DecalComponent))
  (Variables|Material|SetMat_CercleExt _returnvalue)
  (bind _returnvalue_2 (Rendering|Material|CreateDynamicMaterialInstance (Variables|Default|GetRunicExt) :!class /Script/Engine.DecalComponent))
  (Variables|Material|SetMat_RunicExt _returnvalue_2)
  (bind _returnvalue_3 (Rendering|Material|CreateDynamicMaterialInstance (Variables|Default|GetRunicInt) :!class /Script/Engine.DecalComponent))
  (Variables|Material|SetMat_RunicInt _returnvalue_3)
  (bind _returnvalue_4 (Rendering|Material|CreateDynamicMaterialInstance (Variables|Default|GetLogoLegion) :!class /Script/Engine.DecalComponent))
  (Variables|Material|SetMat_Logo _returnvalue_4)
  (bind _returnvalue_5 (Rendering|Material|CreateDynamicMaterialInstance (Variables|Default|GetPortal) 0 "/Game/FX/Main_de_Guldan/Portal/InnerPortal_Inst.InnerPortal_Inst" "None" :!class /Script/Engine.PrimitiveComponent))
  (Variables|Material|SetMat_Portal _returnvalue_5)
  (bind _returnvalue_6 (Rendering|Material|CreateDynamicMaterialInstance (Variables|Default|GetCercleIntérieur) :!class /Script/Engine.DecalComponent))
  (Variables|Material|SetMat_CercleInt _returnvalue_6)
  (bind _returnvalue_7 (Rendering|Material|CreateDynamicMaterialInstance (Variables|Default|GetCercleIntCenter) :!class /Script/Engine.DecalComponent))
  (Variables|Material|SetMat_CercleIntCenter _returnvalue_7)
  (bind _returnvalue_8 (Rendering|Material|CreateDynamicMaterialInstance (Variables|Default|GetPortal) 0 0 "None" :!class /Script/Engine.PrimitiveComponent))
  (Variables|Material|SetMat_Portal _returnvalue_8))

(fn UpdateDynamicMat
  (Rendering|Material|SetScalarParameterValue (Variables|Material|GetMat_RunicExt) "Opacity" (Math|Curves|GetFloatValue (Variables|Curve|GetCurveRunicExt) (Variables|Default|GetTime)) :!class /Script/Engine.MaterialInstanceDynamic)
  (Rendering|Material|SetScalarParameterValue (Variables|Material|GetMat_RunicInt) "Opacity" (Math|Curves|GetFloatValue (Variables|Curve|GetCurveRunicInt) (Variables|Default|GetTime)) :!class /Script/Engine.MaterialInstanceDynamic)
  (Rendering|Material|SetScalarParameterValue (Variables|Material|GetMat_Logo) "Opacity" (Math|Curves|GetFloatValue (Variables|Curve|GetCurveLogo) (Variables|Default|GetTime)) :!class /Script/Engine.MaterialInstanceDynamic)
  (Rendering|Material|SetScalarParameterValue (Variables|Material|GetMat_CercleInt) "Time" (Math|Curves|GetFloatValue (Variables|Curve|GetCurveCercleInt) (Variables|Default|GetTime)) :!class /Script/Engine.MaterialInstanceDynamic)
  (Rendering|Material|SetScalarParameterValue (Variables|Material|GetMat_CercleIntCenter) "Time" (Math|Curves|GetFloatValue (Variables|Curve|GetCurveCercleIntCenter) (Variables|Default|GetTime)) :!class /Script/Engine.MaterialInstanceDynamic)
  (Rendering|Material|SetScalarParameterValue (Variables|Material|GetMat_CercleExt) "Time" (Math|Curves|GetFloatValue (Variables|Curve|GetCurveCercleExterieur) (Variables|Default|GetTime)) :!class /Script/Engine.MaterialInstanceDynamic)
  (Rendering|Material|SetScalarParameterValue (Variables|Material|GetMat_Portal) "Radius" (Math|Curves|GetFloatValue (Variables|Curve|GetCurvePortal) (Variables|Default|GetTime)) :!class /Script/Engine.MaterialInstanceDynamic))

(fn SpawnMeteor
  ;[1 1 1] Meteor spawn
  (if (Variables|Meteor|GetIsMeteorSpawned)
    (return true)
    (elif (> (Variables|Default|GetTime) (Variables|Meteor|GetTimeSpawnMeteor))
      (Variables|Meteor|SetIsMeteorSpawned true)
      (bind _returnvalue (Game|SpawnActorfromClass "/Game/FX/Main_de_Guldan/Meteor/DemonicMeteor.DemonicMeteor_C" (Transformation|GetWorldTransform (Variables|Default|GetMeteorStartPoint)) "Undefined" "MultiplyWithRoot" 0 0))
      (bind _output_get (Variables|Meteor|SetMeteor_BP _returnvalue))
      (Transformation|SetActorRotation _output_get (Math|Random|RandomRotator true)))))

(fn MoveMeteor
  (params (DeltalTime :type Float%20%28double-precision%29))
  (Variables|Meteor|SetTimerMeteorTravel (+ (/ DeltalTime (Variables|Meteor|GetMeteorAirTime)) (Variables|Meteor|GetTimerMeteorTravel)))
  (Transformation|SetActorTransform (Variables|Meteor|GetMeteor_BP) (Math|Transform|Lerp(Transform) (Transformation|GetWorldTransform (Variables|Default|GetMeteorStartPoint)) (Transformation|GetWorldTransform (Variables|Default|GetMeteorEndPoint)) (Math|Curves|GetFloatValue (Variables|Meteor|GetCurveMeteorTavel) (Variables|Meteor|GetTimerMeteorTravel)))))

(fn DestroyMeteor
  (if (Variables|Meteor|GetIsMeteorSpawned)
    (if (>= (Variables|Meteor|GetTimerMeteorTravel) 1.0)
      ;[1 1 1] Explosion event
      (CallFunction|SpawnExplosion (Transformation|GetActorLocation (Variables|Meteor|GetMeteor_BP)))
      (Default|LaunchDestroyTimer (Variables|Meteor|GetMeteor_BP) (Variables|Meteor|GetTimeToDestroyMeteor))
      (Variables|Meteor|SetIsMeteorSpawned false))))

(fn SpawnBeam
  (params (DeltaTime :type Float%20%28double-precision%29))
  (bind _felbeam (Variables|Default|GetFelBeam))
  (bind _screamingsouls (Variables|Default|GetScreamingSouls))
  (if (Variables|Beam|GetHasBeamSpawned)
    (if (<= (Variables|Beam|GetTimerBeam) 1.0)
      (Variables|Beam|SetTimerBeam (+ (/ DeltaTime (Variables|Beam|GetTransitionBeam)) (Variables|Beam|GetTimerBeam)))
      (Effects|Components|ParticleSystem|SetVectorParameter (Variables|Default|GetFelBeam) "EndPoint" (Math|Vector|Lerp(Vector) "0, 0, 0" (- (Transformation|GetWorldLocation (Variables|Default|GetPortal%20Pos)) (Transformation|GetWorldLocation (Variables|Default|GetDefaultSceneRoot))) (Math|Curves|GetFloatValue (Variables|Curve|GetBeamCurve) (Variables|Beam|GetTimerBeam))))
      (if (!= (Variables|Beam|GetHasBeamSpawned) true) :!label _label
        (if (>= (Variables|Default|GetTime) (Variables|Beam|GetTimeBeam))
          (Variables|Beam|SetHasBeamSpawned true)
          (Effects|Components|ParticleSystem|SetVectorParameter _screamingsouls "EndPoint" (- (Transformation|GetWorldLocation (Variables|Default|GetPortal%20Pos)) (Transformation|GetWorldLocation (Variables|Default|GetDefaultSceneRoot))))
          (Components|Activation|Activate _screamingsouls false)
          (Effects|Components|ParticleSystem|SetFloatParameter _felbeam "Duration" (Variables|Beam|GetTransitionBeam))
          (Components|Activation|Activate _felbeam false))))
    (else
      (goto _label))))

(fn CheckAutoDestroy
  (if (>= (Variables|Default|GetTime) (Variables|Default|GetAutoDestroyTime))
    (Actor|DestroyActor)))