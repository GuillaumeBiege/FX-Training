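; Telluric teleportation effect actor that animates a Patatoide mesh and a Sphere component over time.
; BeginPlay creates a dynamic material instance on Patatoide.
; While BoolAnimPata is true, Tick advances a timer that samples curves for the material's color and emissive power and for both components' scales.
; The file never sets that flag or resets the timer.
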(event EventBeginPlay
  (bind _returnvalue (Rendering|Material|CreateDynamicMaterialInstance (Variables|Default|GetPatatoide) 0 "/Game/FX/TelluricTeleportation/PatatoideTransformation/Patatoide_effect_Inst.Patatoide_effect_Inst" "None" :!class /Script/Engine.PrimitiveComponent))
  (Variables|Patatoide|SetPatatoide_Mat _returnvalue))

(event Collision|EventActorBeginOverlap
  (params (OtherActor :type Actor%20Object%20Reference)))

(event EventTick
  (params (DeltaSeconds :type Float%20%28single-precision%29))
  (if (Variables|Patatoide|GetBool_Anim_Pata)
    (bind _output_get (Variables|Patatoide|SetTimer_Pata (+ (Variables|Patatoide|GetTimer_Pata) DeltaSeconds)))
    (Rendering|Material|SetVectorParameterValue (Variables|Patatoide|GetPatatoide_Mat) "MainColor" (Math|Curves|GetLinearColorValue (Variables|Patatoide|GetColorCurve_Pata) _output_get) :!class /Script/Engine.MaterialInstanceDynamic)
    (Audio|Parameter|SetFloatParameter (Variables|Patatoide|GetPatatoide_Mat) "EmissivePower" (Math|Curves|GetFloatValue (Variables|Patatoide|GetEmissiveCurve_Pata) _output_get) :!class /Script/AudioExtensions.AudioParameterControllerInterface)
    (Transformation|SetRelativeScale3D (Variables|Default|GetPatatoide) (Math|Curves|GetVectorValue (Variables|Patatoide|GetScaleCurve_Pata) _output_get))
    (Transformation|SetRelativeScale3D (Variables|Default|GetSphere) (Math|Curves|GetVectorValue (Variables|Sphere|GetScaleCurve_Sphere) _output_get))))

(fn ConstructionScript)